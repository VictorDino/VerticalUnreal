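; Collectable actor that the player picks up by pressing F while standing inside its Box trigger.
; Box overlap with the third-person character enables input on this actor, and end overlap disables it.
; Pressing F decrements CollectablesLeft on BP_ThirdPersonGameMode, shows a new CollectableWidget, calls its Aabar function, then destroys the actor.
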(event `Key|F`
  (params (Key :type "Key Structure"))
  (:`Pressed`
    (bind _asbp_third_person_game_mode (cast `/Game/ThirdPerson/Blueprints/BP_ThirdPersonGameMode` (`GameplayStatics.GetGameMode`)))
    (bind _result (`/Engine/EditorBlueprintResources/StandardMacros.DecrementInt` (`/Game/ThirdPerson/Blueprints/BP_ThirdPersonGameMode.collectables left` _asbp_third_person_game_mode))
      (:`  `
        (set `/Game/ThirdPerson/Blueprints/BP_ThirdPersonGameMode.collectables left` _result _asbp_third_person_game_mode)
        (bind _returnvalue (`|CreateWidget` "/Game/Collectables/CollectableWidget.CollectableWidget_C"))
        (`UserWidget.AddToViewport` _returnvalue 0)
        (`/Game/Collectables/CollectableWidget.Aabar` _returnvalue)
        (`self.K2_DestroyActor`)))))

(event `self.Box.OnComponentBeginOverlap`
  (params (OverlappedComponent :type "PrimitiveComponent Object Reference") (OtherActor :type "Actor Object Reference") (OtherComp :type "PrimitiveComponent Object Reference") (OtherBodyIndex :type Integer) (bFromSweep :type Boolean) (SweepResult :type "HitResult Structure (by ref)"))
  (cast `/Game/ThirdPerson/Blueprints/BP_ThirdPersonCharacter` OtherActor)
  (`self.EnableInput` (`GameplayStatics.GetPlayerController` 0)))

(event `self.Box.OnComponentEndOverlap`
  (params (OverlappedComponent :type "PrimitiveComponent Object Reference") (OtherActor :type "Actor Object Reference") (OtherComp :type "PrimitiveComponent Object Reference") (OtherBodyIndex :type Integer))
  (cast `/Game/ThirdPerson/Blueprints/BP_ThirdPersonCharacter` OtherActor)
  (`self.DisableInput` (`GameplayStatics.GetPlayerController` 0)))

(fn `UserConstructionScript`)